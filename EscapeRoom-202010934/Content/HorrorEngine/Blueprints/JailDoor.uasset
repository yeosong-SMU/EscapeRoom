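; Sliding jail door for HorrorEngine that opens and closes on Use or On/Off interaction events.
; A timeline, rated by a duration setting, lerps the pivot between closed and open locations, with 3D movement and impact sounds.
; A mid-timeline check sets the Open state and fires horror event checks.
; Construction applies meshes and initial position, while save hooks restore the door's state by snapping timeline and pivot.
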(event Custom|OpenDoor
  ;[1 1 1] E-Door Settings
  (Variables|Default|SetOpening true)
  (Utilities|HM3DSound (Variables|E-DoorSettings|GetCloseSound) false (Variables|E-DoorSettings|GetOpenSound) (Variables|Default|GetE-DoorPivot) (Variables|E-DoorSettings|GetSoundAttenuation) 0.0)
  (bind (_direction _animation) (Timeline|OpenCloseTimeline Play)
    (:Update
      (Transformation|SetRelativeLocation (Variables|Default|GetE-DoorPivot) (Math|Vector|Lerp(Vector) (Variables|E-DoorSettings|GetCloseLocation) (Variables|E-DoorSettings|GetOpenLocation) _animation) false false))
    (:Finished
      (switch Utilities|FlowControl|Switch|SwitchonETimelineDirection _direction
        (:Forward
          (Utilities|HM3DSound (Variables|E-DoorSettings|GetOpenSound) false (Variables|E-DoorSettings|GetOpenHitSound) (Variables|Default|GetE-DoorPivot) (Variables|E-DoorSettings|GetSoundAttenuation) 0.0))))
    (:OpenCloseCheck
      (switch Utilities|FlowControl|Switch|SwitchonETimelineDirection _direction
        (:Forward
          (Variables|DoNotChange|SetOpen true)
          (CallFunction|HorrorEventCheck "NewEnumerator3"))
        (:Backward
          (Variables|DoNotChange|SetOpen false)
          (CallFunction|HorrorEventCheck "NewEnumerator4")
          (Utilities|HM3DSound (Variables|E-DoorSettings|GetCloseSound) false (Variables|E-DoorSettings|GetCloseHitSound) (Variables|Default|GetE-DoorPivot) (Variables|E-DoorSettings|GetSoundAttenuation) 0.0))))))

(event Custom|ToggleDoor
  ;[1 1 1] E-Door Settings
  (switch Utilities|FlowControl|Switch|SwitchonETimelineDirection (stale Custom|OpenDoor _direction)
    (:Forward
      (CallFunction|CloseDoor false))
    (:Backward
      (CallFunction|OpenDoor))))

(event Custom|CloseDoor
  (params (Lock :type Boolean))
  ;[1 1 1] E-Door Settings
  (Variables|Default|SetOpening false)
  (Utilities|HM3DSound (Variables|E-DoorSettings|GetOpenSound) false (Variables|E-DoorSettings|GetCloseSound) (Variables|Default|GetE-DoorPivot) (Variables|E-DoorSettings|GetSoundAttenuation) 0.0)
  (bind (_direction _animation) (Timeline|OpenCloseTimeline Reverse)
    (:Update
      (Transformation|SetRelativeLocation (Variables|Default|GetE-DoorPivot) (Math|Vector|Lerp(Vector) (Variables|E-DoorSettings|GetCloseLocation) (Variables|E-DoorSettings|GetOpenLocation) _animation) false false))
    (:Finished
      (switch Utilities|FlowControl|Switch|SwitchonETimelineDirection _direction
        (:Forward
          (Utilities|HM3DSound (Variables|E-DoorSettings|GetOpenSound) false (Variables|E-DoorSettings|GetOpenHitSound) (Variables|Default|GetE-DoorPivot) (Variables|E-DoorSettings|GetSoundAttenuation) 0.0))))
    (:OpenCloseCheck
      (switch Utilities|FlowControl|Switch|SwitchonETimelineDirection _direction
        (:Forward
          (Variables|DoNotChange|SetOpen true)
          (CallFunction|HorrorEventCheck "NewEnumerator3"))
        (:Backward
          (Variables|DoNotChange|SetOpen false)
          (CallFunction|HorrorEventCheck "NewEnumerator4")
          (Utilities|HM3DSound (Variables|E-DoorSettings|GetCloseSound) false (Variables|E-DoorSettings|GetCloseHitSound) (Variables|Default|GetE-DoorPivot) (Variables|E-DoorSettings|GetSoundAttenuation) 0.0))))))

(event EventUse
  (params (HorrorEvent :type Boolean))
  ;[1 1 1] Use / Alternative Use Settings
  (Utilities|HMCheckInteraction)
  (if (Variables|DoNotChange|GetOpen)
    (CallFunction|Close/Off false)
    (else
      (CallFunction|Open/On false))))

(event EventRestoreSaveData
  (params (AssetSave :type Assets%20Save%20Structure))
  ;[0 1 0.5572] Save Settings
  (|BreakAssetSave AssetSave)
  (Components|Timeline|SetNewTime (Variables|Default|GetOpenCloseTimeline) (select (Variables|DoNotChange|GetOpen) 1.0 0.0))
  (Transformation|SetRelativeLocation (Variables|Default|GetE-DoorPivot) (select (Variables|DoNotChange|GetOpen) (Variables|E-DoorSettings|GetOpenLocation) (Variables|E-DoorSettings|GetCloseLocation)) false false))

(event EventBeginLoad
  (Variables|Default|SetOpening (Variables|DoNotChange|GetOpen)))

(event EventCollectSaveData
  ;[0 1 0.5572] Save Settings
  (bind _asmaster (CallFunction|GetPlayer))
  (Utilities|Array|Add (Variables|/Game/HorrorEngine/Blueprints/Core/HE_SaveGameComponent.HE_SaveGameComponent_C|GetAssetCache (Variables|/Game/HorrorEngine/HorrorEngine.HorrorEngine_C|GetHE_SaveGameComponent _asmaster)) (|MakeAssetSave)))

(event EventOpen/On
  (params (HorrorEvent :type Boolean))
  ;[1 1 1] Open / Close Settings
  (Utilities|HMCheckInteraction)
  (if (Variables|DoNotChange|GetOpen)
    (CallFunction|ToggleDoor)
    (else
      (CallFunction|OpenDoor))))

(event EventClose/Off
  (params (HorrorEvent :type Boolean))
  ;[1 1 1] Open / Close Settings
  (Utilities|HMCheckInteraction)
  (if (Variables|DoNotChange|GetOpen)
    (CallFunction|ToggleDoor)))

(fn ConstructionScript
  (Utilities|HMDefaultConstructions (Variables|HorrorEvents|GetCreateNewHorrorEvent))
  (CallFunction|SetMesh (Variables|Default|GetE-Door) (Variables|MeshSettings|GetE-DoorMesh))
  (CallFunction|SetMesh (Variables|Default|GetE-DoorFrame) (Variables|MeshSettings|GetE-DoorFrameMesh))
  (CallFunction|PlayRate (Variables|Default|GetOpenCloseTimeline) (Variables|E-DoorSettings|GetOpen%20/%20Close%20Duration%20%28Sec%29))
  (CallFunction|RefreshDoor))

(fn RefreshDoor
  (Components|Timeline|SetNewTime (Variables|Default|GetOpenCloseTimeline) (select (Variables|DoNotChange|GetOpen) 1.0 0.0))
  (Transformation|SetRelativeLocation (Variables|Default|GetE-DoorPivot) (select (Variables|DoNotChange|GetOpen) (Variables|E-DoorSettings|GetOpenLocation) (Variables|E-DoorSettings|GetCloseLocation)) false false))